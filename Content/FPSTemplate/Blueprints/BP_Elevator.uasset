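; Interactable elevator that soldiers toggle between fully lowered and fully raised, using their push montage.
; Each interaction flips the direction and opens a Tick gate, which moves the clamped height at constant speed until either limit closes it.
; A RepNotify function applies the height, plus a fixed offset, to the platform's relative Z, keeping visual movement separate from the height update.
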(event EventOnInteract
  (params (Soldier :type Soldier%20Object%20Reference))
  (Variables|Default|SetbGoUp (not (Variables|Default|GetbGoUp)))
  (Utilities|FlowControl|Gate true) ; enters at Open
)

(event EventTick
  (params (DeltaSeconds :type Float%20%28single-precision%29))
  (bind _elevationspeed (Variables|Default|GetElevationSpeed))
  (bind _returnvalue (* DeltaSeconds _elevationspeed))
  (Utilities|FlowControl|Gate true :!label _label
    (:Exit
      (bind _output_get (Variables|Default|SetElevationHeight (Math|Float|Clamp(Float) (+ (Variables|Default|GetElevationHeight) (Math|Float|SelectFloat _returnvalue (* _returnvalue -1.0) (Variables|Default|GetbGoUp))) 0.0 (Variables|Default|GetMaxElevationHeight))))
      (if (or (== _output_get 0.0) (== _output_get (Variables|Default|GetMaxElevationHeight)))
        (goto _label Close)))))

(fn ConstructionScript)

(fn K2GetInteractionLength
  (return 0.3))

(fn K2GetInteractionLocation
  (return (Transformation|GetWorldLocation (Variables|Default|GetScene))))

(fn K2CanSoldierInteract
  (params (Soldier :type Soldier%20Object%20Reference))
  (return true))

(fn OnRepElevationRatio
  (Transformation|SetRelativeLocation (Variables|Default|GetPlatform) (Math|Vector|MakeVector 0.0 0.0 (+ (Variables|Default|GetElevationHeight) 1.5e+02)) false false))

(fn K2GetInteractionMontage
  (params (Soldier :type Soldier%20Object%20Reference))
  (return (Variables|/Script/FPSTemplate.Soldier|GetPushMontage Soldier)))
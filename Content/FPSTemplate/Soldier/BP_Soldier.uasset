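; BP_Soldier is a soldier Blueprint that equips a bow and lets input show or remove a pocketknife.
; On BeginPlay it spawns the bow and snaps it to the mesh's grip socket.
; The "visible" action spawns a knife on KnifeSocket, while "invisible" destroys it rather than hiding it.
; The Alreadyspawned flag prevents duplicate knives, and Kk keeps the reference for removal.
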(event EventBeginPlay
  (Utilities|FlowControl|Sequence
    (:then_0
      (bind _returnvalue (Game|SpawnActorfromClass "/Game/FPSTemplate/Items/Bow_bp2.Bow_bp2_C" (Math|Transform|MakeTransform "0, 0, 0") "AlwaysSpawn" 0 0))
      (Transformation|AttachComponentToComponent _returnvalue (Variables|Character|GetMesh) "grip" "SnapToTarget" "SnapToTarget" "SnapToTarget" true))))

(event Input|ActionEvents|InputActionvisible
  (params (Key :type Key%20Structure))
  (:Pressed
    (if (not (Variables|Default|Getalreadyspawned))
      (bind _returnvalue (Game|SpawnActorfromClass "/Game/FPSTemplate/Items/M9/pocketknife.pocketknife_C" (Math|Transform|MakeTransform "0, 0, 0") "AlwaysSpawn" 0 0))
      (bind _output_get (Variables|Default|Setkk _returnvalue))
      (Transformation|AttachComponentToComponent _output_get (Variables|Character|GetMesh) "KnifeSocket" "SnapToTarget" "SnapToTarget" "SnapToTarget" true)
      (Variables|Default|Setalreadyspawned true))))

(event Input|ActionEvents|InputActioninvisible
  (params (Key :type Key%20Structure))
  (:Pressed
    (if (Variables|Default|Getalreadyspawned)
      (Actor|DestroyActor (Variables|Default|Getkk))
      (Variables|Default|Setalreadyspawned false))))

(fn ConstructionScript)